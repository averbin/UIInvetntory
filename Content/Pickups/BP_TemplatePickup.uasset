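; Template pickup actor that the player can collect into the HUD inventory and later use to add health, energy and mood.
; The construction script applies a custom mesh and fills the item struct with image, pickup text and action text.
; A trigger overlap shows a prompt widget and marks it in range, enabling a handler bound through the first-person character.
; Pickup hides the actor rather than destroying it; UseAction applies the stats and destroys it.
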(event `self.ReceiveBeginPlay`
  (bind _iteminfo (`self.ItemInfo`))
  (bind _pickuptextref (`self.PickupTextRef`))
  (bind (_item _itemimage _pickuptext) (break `/Game/FirstPersonBP/Blueprints/InventoryStruct` _iteminfo))
  ;[1 1 1] Event Begin Play
  (bind _returnvalue (`|CreateWidget` "/Game/UMG/PickupText.PickupText_C"))
  (set `self.PickupTextRef` _returnvalue)
  (setmembers `/Game/FirstPersonBP/Blueprints/InventoryStruct` :`StructRef` _iteminfo :`Item` self)
  (set `PickupWidget.PickupActor` _item _pickuptextref)
  (set `/Game/UMG/PickupText.PickupText` _pickuptext _pickuptextref)
  (bind _asfirst_person_character (cast `/Game/FirstPersonBP/Blueprints/FirstPersonCharacter` (`GameplayStatics.GetPlayerCharacter` 0)))
  (bind _output_get (set `self.CharacterRef` _asfirst_person_character))
  (add `/Game/FirstPersonBP/Blueprints/FirstPersonCharacter.PickupItem` _output_get (delegate `PickupItem_Event_0`)))

(event `PickupItem_Event_0`
  (bind _gamehudref (`/Game/FirstPersonBP/Blueprints/FirstPersonCharacter.GameHUDRef` (`self.CharacterRef`)))
  ;[1 1 1] Pickup and Add Item to an Inventory then refresh it
  (if (and (`self.GetActorEnableCollision`) (`self.IsInRange?`))
    (`KismetArrayLibrary.Array_Add` (`/Game/UMG/GameHUD.Inventory` _gamehudref) (`self.ItemInfo`))
    (`Widget.RemoveFromParent` (`self.PickupTextRef`))
    (`self.SetActorHiddenInGame` true)
    (`self.SetActorEnableCollision` false)
    (`/Game/UMG/GameHUD.RefreshInventory` _gamehudref)))

(event `self.Trigger.OnComponentBeginOverlap`
  (params (OverlappedComponent :type "PrimitiveComponent Object Reference") (OtherActor :type "Actor Object Reference") (OtherComp :type "PrimitiveComponent Object Reference") (OtherBodyIndex :type Integer) (bFromSweep :type Boolean) (SweepResult :type "HitResult Structure (by ref)"))
  ;[1 1 1] Overlap Trigger Script
  (cast `/Game/FirstPersonBP/Blueprints/FirstPersonCharacter` OtherActor)
  (`UserWidget.AddToViewport` (`self.PickupTextRef`) 0)
  (set `self.IsInRange?` true))

(event `self.Trigger.OnComponentEndOverlap`
  (params (OverlappedComponent :type "PrimitiveComponent Object Reference") (OtherActor :type "Actor Object Reference") (OtherComp :type "PrimitiveComponent Object Reference") (OtherBodyIndex :type Integer))
  ;[1 1 1] Overlap Trigger Script
  (cast `/Game/FirstPersonBP/Blueprints/FirstPersonCharacter` OtherActor)
  (`Widget.RemoveFromParent` (`self.PickupTextRef`))
  (set `self.IsInRange?` false))

(event `/Game/FirstPersonBP/Blueprints/ActionInterface.UseAction`
  (bind _characterref (`self.CharacterRef`))
  ;[1 1 1] Use Action
  (set `CharacterBase.HealthValue` (+ (`CharacterBase.HealthValue` _characterref) (`self.AddHealth`)) _characterref)
  (set `CharacterBase.EnergyValue` (+ (`CharacterBase.EnergyValue` _characterref) (`self.AddEnergy`)) _characterref)
  (set `CharacterBase.MoodValue` (+ (`CharacterBase.MoodValue` _characterref) (`self.AddMood`)) _characterref)
  (`self.K2_DestroyActor`))

(fn `UserConstructionScript`
  (setmembers `/Game/FirstPersonBP/Blueprints/InventoryStruct` :`StructRef` (`self.ItemInfo`) :`Item` self :`ItemImage` (`self.CustomPickupImage`) :`PickupText` (`self.CustomPickupText`) :`ActionText` (`self.CustomActionText`))
  (`StaticMeshComponent.SetStaticMesh` (`self.StaticMesh`) (`self.CustomMesh`)))